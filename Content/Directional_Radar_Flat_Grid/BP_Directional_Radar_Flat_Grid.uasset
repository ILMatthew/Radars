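; Directional flat-grid radar actor that animates a back-and-forth scan over a limited horizontal angle, with clamped or auto-cycled vertical inclination.
; A timeline and timers drive the sweep, writing scan position, inclination and angle into packed channels of a material parameter collection vector.
; A dot-product cone test maps contacts into radar space.
; An input-moved Niagara cursor picks contacts, debug-printed each tick in one of two colors.
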(event `self.ReceiveBeginPlay`
  (`parent.ReceiveBeginPlay`)
  (`self.SetAnimSpeed`)
  (`KismetSystemLibrary.K2_SetTimerDelegate` (`|CreateDelegate` :!event `AnimateRadar`) (`self.TimeBetweenUpdates`))
  (`self.SetHorizontalAngle` (`self.HorizontalAngle`)))

(event `self.ReceiveTick`
  (params (DeltaSeconds :type "Float (single-precision)"))
  (`parent.ReceiveTick` DeltaSeconds)
  (`self.PrintSelectedTarget`))

(event `AnimateRadar`
  (switch `ETimelineDirection` (stale _direction)
    (:`Forward`
      (bind (_direction _alpha) (`Timeline|HorizontalScan` :!via `Reverse` :!label _label)
        (:`Update`
          (bind _returnvalue (`KismetMaterialLibrary.GetVectorParameterValue` "/Radars/Directional_Radar_Flat_Grid/DirectionalRadar_Grid_Collection.DirectionalRadar_Grid_Collection" "Controls"))
          (bind (_r _g _b _a) (`KismetMathLibrary.BreakColor` _returnvalue))
          (bind _returnvalue_2 (- _b 0.05))
          (`KismetMaterialLibrary.SetVectorParameterValue` "/Radars/Directional_Radar_Flat_Grid/DirectionalRadar_Grid_Collection.DirectionalRadar_Grid_Collection" "Controls" (`KismetMathLibrary.MakeColor` (`KismetMathLibrary.Lerp` _returnvalue_2 (* _returnvalue_2 -1.0) _alpha) _g _b _a)))
        (:`Finished`
          (`KismetSystemLibrary.K2_SetTimerDelegate` (`|CreateDelegate` :!event `AnimateRadar`) (`self.TimeBetweenUpdates`))
          (`self.SetVerticalIncl` 0.0))))
    (:`Backward`
      (goto _label))))

(fn `AngleToDot`
  (params (Angle :type "Float (double-precision)"))
  (returns (Dot :type "Float (double-precision)"))
  (return (- 1.0 (/ (/ Angle 2.0) 90.0))))

(fn `ChangeHorizontalAngle`
  (`self.SetHorizontalAngle` (select `int` (`self.testHorizontal`) :`0` 120.0 :`1` 45.0 :`2` 30.0))
  (bind _result (`/Engine/EditorBlueprintResources/StandardMacros.IncrementInt` (`self.testHorizontal`))
    (:`  `
      (if (> _result 2)
        (set `self.testHorizontal` 0)))))

(fn `MapContactLocation`
  (params (ContactLocation :type "Vector Structure") (ContactDirection :type "Rotator Structure"))
  (returns (bIsInsideRadar :type Boolean) (LocationOnRadar :type "Vector Structure") (Angle :type "Float (double-precision)"))
  (bind (_returnvalue_roll _returnvalue_pitch _returnvalue_yaw) (`KismetMathLibrary.BreakRotator` (`KismetMathLibrary.InverseTransformRotation` (`self.GetTransform`) ContactDirection)))
  (bind _returnvalue (- ContactLocation (`self.K2_GetActorLocation`)))
  (bind (_x _y _z) (`KismetMathLibrary.BreakVector3f` (/ (`KismetMathLibrary.InverseTransformDirection` (`self.GetTransform`) _returnvalue) (`self.RadarMaxDistance`))))
  (if (> (`KismetMathLibrary.Dot_VectorVector` (`KismetMathLibrary.Normal` _returnvalue) (`self.GetActorForwardVector`)) (`self.AngleToDot` (`self.HorizontalAngle`)))
    (return true (`KismetMathLibrary.MakeVector` (* (- (* _x 2.0) 1.0) (`self.RadarScale`)) _y _z) _returnvalue_yaw)
    (else
      (return false (0.0 0.0 0.0) 0.0))))

(fn `MoveCursor`
  (params (Input :type "Vector2D Structure"))
  (bind _output_get (set `self.CursorLoc` (`KismetMathLibrary.ClampAxes2D` (+ (* Input (`self.CursorSpeed`) (`GameplayStatics.GetWorldDeltaSeconds`)) (`self.CursorLoc`)) -0.95 0.95)))
  (`NiagaraComponent.SetVariableVec3` (`self.Niagara`) "CursorLocation" (`KismetMathLibrary.MakeVector` (`KismetMathLibrary.BreakVector2D` _output_get) (`.Y` (`KismetMathLibrary.BreakVector2D` _output_get)) 0.001)))

(fn `PrintSelectedTarget`
  (bind _returnvalue (/ 1.0 20.0))
  (bind _returnvalue_2 (/ 1.0 20.0))
  (bind (_cursorloc_x _cursorloc_y) (`KismetMathLibrary.BreakVector2D` (`self.CursorLoc`)))
  (bind _cursorloc_x_2 (`KismetMathLibrary.BreakVector2D` (`self.CursorLoc`)))
  (for (_array_element _array_index) (`self.ContactLocations`)
    (if (and (`KismetMathLibrary.InRange_FloatFloat` (.x _array_element) (+ _cursorloc_x_2 (* _returnvalue_2 -1.0)) (+ _cursorloc_x_2 _returnvalue_2) false false) (`KismetMathLibrary.InRange_FloatFloat` (.y _array_element) (+ _cursorloc_y (* _returnvalue -1.0)) (+ _cursorloc_y _returnvalue) false false))
      (`|ExecutionSequence`
        (:`then_0`
          (break))
        (:`then_1`
          (bind (_output_x _output_y) (`KismetMathLibrary.BreakVector2D` (`|GetArrayItem` (`self.ContactInfos`) _array_index)))
          (`KismetSystemLibrary.PrintString` (`KismetStringLibrary.Conv_VectorToString` (`KismetMathLibrary.MakeVector` (.x _array_element) (.y _array_element) (.z _array_element))) true true (`KismetMathLibrary.SelectColor` (struct :`R` 1.0 :`A` 1.0) (struct :`G` 0.620584 :`B` 1.0 :`A` 1.0) (`KismetMathLibrary.Conv_IntToBool` (`KismetMathLibrary.FFloor` _output_y))) 0.01))))))

(fn `SetAnimSpeed`
  (`TimelineComponent.SetPlayRate` (`self.HorizontalScan`) (/ 1.0 (/ (`self.HorizontalAngle`) (`self.HorizontalSpeed`)))))

(fn `SetHorizontalAngle`
  (params (NewAngle :type "Float (double-precision)"))
  (set `self.HorizontalAngle` NewAngle)
  (bind _returnvalue (`KismetMaterialLibrary.GetVectorParameterValue` "/Radars/Directional_Radar_Flat_Grid/DirectionalRadar_Grid_Collection.DirectionalRadar_Grid_Collection" "Controls"))
  (bind (_r _g _b _a) (`KismetMathLibrary.BreakColor` _returnvalue))
  (`KismetMaterialLibrary.SetVectorParameterValue` "/Radars/Directional_Radar_Flat_Grid/DirectionalRadar_Grid_Collection.DirectionalRadar_Grid_Collection" "Controls" (`KismetMathLibrary.MakeColor` _r _g (/ (`self.HorizontalAngle`) 120.0) _a))
  (`self.SetAnimSpeed`))

(fn `SetVerticalIncl`
  (params (NewIncl :type "Float (double-precision)"))
  (bind _maxverticalincl (`self.MaxVerticalIncl`))
  (bind _maxverticalincl_2 (`self.MaxVerticalIncl`))
  (bind _maxverticalincl_3 (`self.MaxVerticalIncl`))
  (if (`self.bVerticalIsAuto`)
    (set `self.VerticalIncl` (select `int` (`self.CurrentInclSetting`) :`0` _maxverticalincl :`1` 0.0 :`2` (* _maxverticalincl -1.0)))
    (bind _result (`/Engine/EditorBlueprintResources/StandardMacros.IncrementInt` (`self.CurrentInclSetting`))
      (:`  `
        (if (> _result 2)
          (set `self.CurrentInclSetting` 0))))
    (else
      (set `self.CurrentInclSetting` 0)
      (set `self.VerticalIncl` (`KismetMathLibrary.FClamp` NewIncl (* _maxverticalincl_3 -1.0) _maxverticalincl_3))))
  (bind _returnvalue (`KismetMaterialLibrary.GetVectorParameterValue` "/Radars/Directional_Radar_Flat_Grid/DirectionalRadar_Grid_Collection.DirectionalRadar_Grid_Collection" "Controls"))
  (bind (_r _g _b _a) (`KismetMathLibrary.BreakColor` _returnvalue))
  (`KismetMaterialLibrary.SetVectorParameterValue` "/Radars/Directional_Radar_Flat_Grid/DirectionalRadar_Grid_Collection.DirectionalRadar_Grid_Collection" "Controls" (`KismetMathLibrary.MakeColor` _r (`KismetMathLibrary.Lerp` 0.48 0.78 (/ (+ (`self.VerticalIncl`) _maxverticalincl_2) (* _maxverticalincl_2 2.0))) _b _a)))

(fn `UserConstructionScript`
  (`parent.UserConstructionScript`))