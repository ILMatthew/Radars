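; BP_OmnidirectionalRadar_3D is a 3D radar actor that displays surrounding I_Target contacts through Niagara.
; Each tick it sphere-overlaps within RadarRadius, converting contact offsets to local space scaled by the radius.
; Those positions, plus player and enemy flags packed into 2D vectors, feed Niagara array parameters.
; On BeginPlay its SceneCaptureComponent2D adds the radar itself to ShowOnlyActors.
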(event `self.ReceiveBeginPlay`
  (`KismetArrayLibrary.Array_Add` (`SceneCaptureComponent.ShowOnlyActors` (`self.SceneCaptureComponent2D`)) self))

(event `self.ReceiveTick`
  (params (DeltaSeconds :type "Float (single-precision)"))
  (bind _niagara (`self.Niagara`))
  (`KismetArrayLibrary.Array_Clear` (`self.ContactInfo`))
  (`KismetArrayLibrary.Array_Clear` (`self.ContactLocation`))
  (bind (_outactors _returnvalue) (`KismetSystemLibrary.SphereOverlapActors` (`self.K2_GetActorLocation`) (`self.RadarRadius`) (`|MakeArray` "ObjectTypeQuery1" "ObjectTypeQuery2" :!type "EObjectTypeQuery Enum")))
  (if _returnvalue
    (for _array_element _outactors
      (if (`KismetSystemLibrary.DoesImplementInterface` _array_element "/Radars/General/I_Target.I_Target_C")
        (`KismetArrayLibrary.Array_Add` (`self.ContactLocation`) (/ (`KismetMathLibrary.InverseTransformDirection` (`self.GetTransform`) (- (`self.K2_GetActorLocation` _array_element) (`self.K2_GetActorLocation`))) (`self.RadarRadius`)))
        (bind _bisplayer (message `/Radars/General/I_Target.IsPlayer` _array_element))
        (bind _bisenemy (message `/Radars/General/I_Target.IsEnemy` _array_element))
        (`KismetArrayLibrary.Array_Add` (`self.ContactInfo`) (`KismetMathLibrary.MakeVector2D` (`KismetMathLibrary.Conv_BoolToDouble` _bisplayer) (`KismetMathLibrary.Conv_BoolToDouble` _bisenemy)))))
    (`NiagaraDataInterfaceArrayFunctionLibrary.SetNiagaraArrayVector` _niagara "ContactLocations" (`self.ContactLocation`))
    (`NiagaraDataInterfaceArrayFunctionLibrary.SetNiagaraArrayVector2D` _niagara "ContactInfo" (`self.ContactInfo`))))

(fn `UserConstructionScript`)