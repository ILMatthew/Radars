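; Omnidirectional radar actor with a flat top-down display, supplying the mapping from world contacts to radar positions.
; MapContactLocation rotates the offset from the actor into its local space and divides by RadarMaxDistance for X and Y, flattening Z to zero.
; It returns the contact direction's local yaw as the angle and always reports the contact as inside the radar, with no range check.
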(fn `MapContactLocation`
  (params (ContactLocation :type "Vector Structure") (ContactDirection :type "Rotator Structure"))
  (returns (bIsInsideRadar :type Boolean) (LocationOnRadar :type "Vector Structure") (Angle :type "Float (double-precision)"))
  (bind _returnvalue (`self.GetTransform`))
  (bind (_returnvalue_roll _returnvalue_pitch _returnvalue_yaw) (`KismetMathLibrary.BreakRotator` (`KismetMathLibrary.InverseTransformRotation` _returnvalue ContactDirection)))
  (bind (_returnvalue_x _returnvalue_y) (`KismetMathLibrary.BreakVector` (/ (`KismetMathLibrary.InverseTransformDirection` _returnvalue (- ContactLocation (`self.K2_GetActorLocation`))) (`self.RadarMaxDistance`))))
  (return true (`KismetMathLibrary.MakeVector` _returnvalue_x _returnvalue_y) _returnvalue_yaw))

(fn `UserConstructionScript`
  (`parent.UserConstructionScript`))