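; BP_DirectionalRadar_Flat is an actor that maps world contacts onto a flat, forward-facing radar.
; MapContactLocation rejects contacts outside the ScanAngle cone using a dot product threshold from AngleToDot, a linear conversion rather than cosine.
; Accepted contacts become actor-local offsets scaled by RadarMaxDistance and remapped to 2D radar coordinates, with relative yaw for heading.
; Distance is never clamped, and the event graph is unused.
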(fn `AngleToDot`
  (params (Angle :type "Float (double-precision)"))
  (returns (Dot :type "Float (double-precision)"))
  (return (- 1.0 (/ (/ Angle 2.0) 90.0))))

(fn `MapContactLocation`
  (params (ContactLocation :type "Vector Structure") (ContactDirection :type "Rotator Structure"))
  (returns (bIsInsideRadar :type Boolean) (LocationOnRadar :type "Vector Structure") (Angle :type "Float (double-precision)"))
  (bind (_returnvalue_roll _returnvalue_pitch _returnvalue_yaw) (`KismetMathLibrary.BreakRotator` (`KismetMathLibrary.InverseTransformRotation` (`self.GetTransform`) ContactDirection)))
  (bind _returnvalue (- ContactLocation (`self.K2_GetActorLocation`)))
  (bind (_x _y _z) (`KismetMathLibrary.BreakVector3f` (/ (`KismetMathLibrary.InverseTransformDirection` (`self.GetTransform`) _returnvalue) (`self.RadarMaxDistance`))))
  (bind _returnvalue_2 (`KismetMathLibrary.MakeVector` _x _y _z))
  (bind _returnvalue_x (`KismetMathLibrary.BreakVector` (- (* _returnvalue_2 2.0) 1.0)))
  (bind (_returnvalue_x_2 _returnvalue_y) (`KismetMathLibrary.BreakVector` (+ (* _returnvalue_2 0.5) 0.5)))
  (if (> (`KismetMathLibrary.Dot_VectorVector` (`KismetMathLibrary.Normal` _returnvalue) (`self.GetActorForwardVector`)) (`self.AngleToDot` (`self.ScanAngle`)))
    (return true (`KismetMathLibrary.MakeVector` _returnvalue_x (`KismetMathLibrary.Lerp` -1.0 1.0 _returnvalue_y)) _returnvalue_yaw)
    (else
      (return false (0.0 0.0 0.0) 0.0))))

(fn `UserConstructionScript`
  (`parent.UserConstructionScript`))