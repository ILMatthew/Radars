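; Omnidirectional radar actor variant that maps contacts onto a flat, forward-facing 2D display.
; MapContactLocation converts the direction to a contact into the actor's local space, normalizes it and uses its up and right components as radar coordinates.
; Clamping the vector length keeps contacts ahead within an inner disc and pins those behind to an outer ring.
; Every contact reports as inside the radar, regardless of distance.
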(fn `MapContactLocation`
  (params (ContactLocation :type "Vector Structure"))
  (returns (bIsInsideRadar :type Boolean) (LocationOnRadar :type "Vector Structure"))
  (bind (_returnvalue_x _returnvalue_y _returnvalue_z) (`KismetMathLibrary.BreakVector` (`KismetMathLibrary.Normal` (`KismetMathLibrary.InverseTransformDirection` (`self.GetTransform`) (- ContactLocation (`self.K2_GetActorLocation`))))))
  (bind _returnvalue (< _returnvalue_x 0.0))
  (bind (_returnvalue_x_2 _returnvalue_y_2) (`KismetMathLibrary.BreakVector` (`KismetMathLibrary.ClampVectorSize` (`KismetMathLibrary.MakeVector` _returnvalue_z _returnvalue_y) (`KismetMathLibrary.SelectFloat` 0.95 0.0 _returnvalue) (`KismetMathLibrary.SelectFloat` 0.95 0.85 _returnvalue))))
  (return true (`KismetMathLibrary.MakeVector` _returnvalue_x_2 _returnvalue_y_2)))

(fn `UserConstructionScript`
  (`parent.UserConstructionScript`))