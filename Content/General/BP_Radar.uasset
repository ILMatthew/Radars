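; BP_Radar is a radar actor that shows nearby I_Target actors as Niagara contacts.
; A self-rescheduling timer runs a sphere overlap, gathering locations, angles and player/enemy flags into arrays pushed to Niagara.
; MapContactLocation converts world transforms to radar space, but here it only returns outside-radar defaults.
; With a valid TextureTarget, BeginPlay adds an overhead scene capture with the radar in its show-only list, targeting that texture.
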(event `self.ReceiveBeginPlay`
  (`|ExecutionSequence`
    (:`then_0`
      (`/Engine/EditorBlueprintResources/StandardMacros.IsValid` (`self.Texture Target`)
        (:`Is Valid`
          (`self.CreateSceneCapture`))))
    (:`then_1`
      (`FXSystemComponent.SetFloatParameter` (`self.Niagara`) "TimeToUpdate" (`self.TimeBetweenUpdates`))
      (`self.UpdateRadar`))))

(fn `CreateSceneCapture`
  (bind _returnvalue (`AddComponent|NODE_AddSceneCaptureComponent2D-0` :`RelativeTransform` (`KismetMathLibrary.MakeTransform` (0.0 0.0 250.0) (struct :`Pitch` -90.0))))
  (`KismetArrayLibrary.Array_Add` (`SceneCaptureComponent.ShowOnlyActors` _returnvalue) self)
  (set `SceneCaptureComponent2D.TextureTarget` (`self.Texture Target`) _returnvalue))

(fn `MapContactLocation`
  (params (ContactLocation :type "Vector Structure") (ContactDirection :type "Rotator Structure"))
  (returns (bIsInsideRadar :type Boolean) (LocationOnRadar :type "Vector Structure") (Angle :type "Float (double-precision)"))
  (return false (0.0 0.0 0.0) 0.0))

(fn `UpdateNiagara`
  (bind _niagara (`self.Niagara`))
  (`NiagaraDataInterfaceArrayFunctionLibrary.SetNiagaraArrayVector` _niagara "ContactLocations" (`self.ContactLocations`))
  (`NiagaraDataInterfaceArrayFunctionLibrary.SetNiagaraArrayVector2D` _niagara "ContactInfo" (`self.ContactInfos`))
  (`NiagaraDataInterfaceArrayFunctionLibrary.SetNiagaraArrayFloat` _niagara "ContactAngles" (`self.ContactAngles`)))

(fn `UpdateRadar`
  (`KismetArrayLibrary.Array_Clear` (`self.ContactLocations`))
  (`KismetArrayLibrary.Array_Clear` (`self.ContactInfos`))
  (`KismetArrayLibrary.Array_Clear` (`self.ContactAngles`))
  (bind (_outactors _returnvalue) (`KismetSystemLibrary.SphereOverlapActors` (`self.K2_GetActorLocation`) (`self.RadarMaxDistance`) (`|MakeArray` "ObjectTypeQuery1" "ObjectTypeQuery2" :!type "EObjectTypeQuery Enum")))
  (if _returnvalue
    (for _array_element _outactors
      (if (`KismetSystemLibrary.DoesImplementInterface` _array_element "/Radars/General/I_Target.I_Target_C")
        (bind (_bisinsideradar _locationonradar _angle) (`self.MapContactLocation` (`self.K2_GetActorLocation` _array_element) (`self.K2_GetActorRotation` _array_element)))
        (if _bisinsideradar
          (`KismetArrayLibrary.Array_Add` (`self.ContactLocations`) _locationonradar)
          (`KismetArrayLibrary.Array_Add` (`self.ContactAngles`) _angle)
          (bind _bisplayer (message `/Radars/General/I_Target.IsPlayer` _array_element))
          (bind _bisenemy (message `/Radars/General/I_Target.IsEnemy` _array_element))
          (`KismetArrayLibrary.Array_Add` (`self.ContactInfos`) (`KismetMathLibrary.MakeVector2D` (`KismetMathLibrary.Conv_BoolToDouble` _bisplayer) (`KismetMathLibrary.Conv_BoolToDouble` _bisenemy))))))
    (`self.UpdateNiagara`))
  (`KismetSystemLibrary.K2_SetTimer` null "UpdateRadar" (`self.TimeBetweenUpdates`)))

(fn `UserConstructionScript`)